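; Template inventory pickup actor that the player collects in range and later uses to add Health and Energy.
; BeginPlay creates the prompt widget and binds pickup to MyCharacter's PickupItem dispatcher; trigger overlaps toggle the prompt and range flag.
; Pickup adds ItemInfo to the HUD inventory, refreshes it and hides the actor, but leaves collision enabled.
; UseAction applies the stat bonuses and destroys the actor.
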(event `self.ReceiveBeginPlay`
  (bind _iteminfo (`self.ItemInfo`))
  (bind _pickuptextref (`self.PickupTextRef`))
  (bind (_item _itemimage _pickuptext) (break `/Game/Blueprints/InventoryStructure` _iteminfo))
  ;[1 1 1] Event Begin Play
  (bind _returnvalue (`|CreateWidget` "/Game/Blueprints/UMG/PickupText.PickupText_C"))
  (set `self.PickupTextRef` _returnvalue)
  (setmembers `/Game/Blueprints/InventoryStructure` :`StructRef` _iteminfo :`Item` self)
  (set `/Game/Blueprints/UMG/PickupText.PickupActor` _item _pickuptextref)
  (set `/Game/Blueprints/UMG/PickupText.PickupText` _pickuptext _pickuptextref)
  (bind _asmy_character (cast `/Game/Blueprints/MyCharacter` (`GameplayStatics.GetPlayerCharacter` 0)))
  (bind _output_get (set `self.MyCharacterRef` _asmy_character))
  (add `/Game/Blueprints/MyCharacter.PickupItem` _output_get (delegate `PickupItem_Event_0`)))

(event `self.Trigger.OnComponentBeginOverlap`
  (params (OtherActor :type "Actor Object Reference") (OtherComp :type "PrimitiveComponent Object Reference") (OtherBodyIndex :type Integer) (bFromSweep :type Boolean) (SweepResult :type "HitResult Structure (by ref)"))
  ;[1 1 1] Overlap Trigger Script
  (cast `/Game/Blueprints/MyCharacter` OtherActor)
  (`UserWidget.AddToViewport` (`self.PickupTextRef`) 0)
  (set `self.IsInRange?` true))

(event `PickupItem_Event_0`
  (bind _gamehud_ref (`/Game/Blueprints/MyCharacter.GameHuD_Ref` (`self.MyCharacterRef`)))
  ;[1 1 1] Pickup and add item to inventory then refresh
  (if (and (`self.GetActorEnableCollision`) (`self.IsInRange?`))
    (`KismetArrayLibrary.Array_Add` (`/Game/Blueprints/UMG/GameHUD.Inventory` _gamehud_ref) (`self.ItemInfo`))
    (`Widget.RemoveFromParent` (`self.PickupTextRef`))
    (`self.SetActorHiddenInGame` true)
    (`self.SetActorEnableCollision` true)
    (`/Game/Blueprints/UMG/GameHUD.RefreshInventory` _gamehud_ref)))

(event `self.Trigger.OnComponentEndOverlap`
  (params (OtherActor :type "Actor Object Reference") (OtherComp :type "PrimitiveComponent Object Reference") (OtherBodyIndex :type Integer))
  ;[1 1 1] Overlap Trigger Script
  (cast `/Game/Blueprints/MyCharacter` OtherActor)
  (`Widget.RemoveFromParent` (`self.PickupTextRef`))
  (set `self.IsInRange?` false))

(event `/Game/Blueprints/ActionInterface.UseAction`
  (bind _mycharacterref (`self.MyCharacterRef`))
  ;[1 1 1] Use Action
  (set `/Game/Blueprints/MyCharacter.Health` (+ (`/Game/Blueprints/MyCharacter.Health` _mycharacterref) (`self.AddHealth`)) _mycharacterref)
  (set `/Game/Blueprints/MyCharacter.Energy` (+ (`/Game/Blueprints/MyCharacter.Energy` _mycharacterref) (`self.AddEnergy`)) _mycharacterref)
  (`self.K2_DestroyActor`))

(fn `UserConstructionScript`)