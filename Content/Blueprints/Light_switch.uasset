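; Light switch actor that lets the player turn a spot light and a round light on and off with the F key.
; Overlapping the trigger box enables input for player controller 0 and toggles a message's visibility; ending the overlap disables input and toggles it again, with no check on the overlapping actor.
; The construction script applies the LightColor and OnOff variables to both lights as their color and starting visibility.
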(event `self.TriggerBox.OnComponentBeginOverlap`
  (params (OtherActor :type "Actor Object Reference") (OtherComp :type "PrimitiveComponent Object Reference") (OtherBodyIndex :type Integer) (bFromSweep :type Boolean) (SweepResult :type "HitResult Structure (by ref)"))
  (`self.EnableInput` (`GameplayStatics.GetPlayerController` 0))
  (`SceneComponent.ToggleVisibility` (`self.Message`) false :!label _label))

(event `self.ReceiveBeginPlay`)

(event `self.ReceiveActorBeginOverlap`
  (params (OtherActor :type "Actor Object Reference")))

(event `self.TriggerBox.OnComponentEndOverlap`
  (params (OtherActor :type "Actor Object Reference") (OtherComp :type "PrimitiveComponent Object Reference") (OtherBodyIndex :type Integer))
  (`self.DisableInput` (`GameplayStatics.GetPlayerController` 0))
  (goto _label))

(event `self.ReceiveTick`
  (params (DeltaSeconds :type "Float (single-precision)")))

(event `Key|F`
  (:`Pressed`
    (`SceneComponent.ToggleVisibility` (`self.roundLight`) false)
    (`SceneComponent.ToggleVisibility` (`self.SpotLight`) false)))

(fn `UserConstructionScript`
  (`LightComponent.SetLightColor` (`self.SpotLight`) (`self.LightColor`))
  (`LightComponent.SetLightColor` (`self.roundLight`) (`self.LightColor`))
  (`SceneComponent.SetVisibility` (`self.roundLight`) (`self.On/Off`) false)
  (`SceneComponent.SetVisibility` (`self.SpotLight`) (`self.On/Off`) false))